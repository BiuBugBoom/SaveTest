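; BP_GameMode is a Game Mode in the Vehicle folder that handles saving the game.
; SaveGame gets BP_GameInstance, creates a BP_SaveGame object if none is valid, and writes it to the slot name selected by the instance's SaveGameInt.
; LoadGame, RecardGame, ReplayGame and SpawnCar are empty stubs, and BeginPlay, Tick and the construction script do nothing.
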(event EventBeginPlay)

(event EventTick
  (params (DeltaSeconds :type Float%20%28single-precision%29)))

(fn ConstructionScript)

(fn SaveGame
  (bind _asbp_game_instance (Utilities|Casting|CastToBP_GameInstance (Game|GetGameInstance)))
  (Variables|Default|SetBP_GameInstance _asbp_game_instance)
  (Utilities|IsValid (Variables|Default|GetBP_SaveGame)
    (:Is%20Valid
      _)
    (:Is%20Not%20Valid
      (bind _returnvalue (SaveGame|CreateSaveGameObject "/Game/Vehicle/BP_SaveGame.BP_SaveGame_C"))
      (Variables|Default|SetBP_SaveGame _returnvalue)))
  (SaveGame|SaveGametoSlot (Variables|Default|GetBP_SaveGame) (Utilities|Array|Get(acopy) (Variables|Default|GetSlotName) (Variables|/Game/Vehicle/BP_Gameinstance.BP_GameInstance_C|GetSaveGameInt (Variables|Default|GetBP_GameInstance)))))

(fn LoadGame)

(fn RecardGame)

(fn ReplayGame)

(fn SpawnCar)